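; BP_PlayerControl turns input axes into movement and look control for the player's BP_Player pawn.
; On BeginPlay it casts player pawn 0 to BP_Player and caches the reference.
; Move axes feed AddMovementInput along that pawn's forward and right vectors, while Rotate and LookUp feed its controller yaw and pitch input.
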(event EventBeginPlay
  (bind _asbp_player (Utilities|Casting|CastToBP_Player (Game|Player|GetPlayerPawn 0)))
  (Variables|Default|SetAs%20BP%20Player _asbp_player))

(event Input|AxisEvents|InputAxisMoveLeftRight
  (params (AxisValue :type Float%20%28single-precision%29))
  (bind _as_bp_player (Variables|Default|GetAs%20BP%20Player))
  ;[1 1 1] Move
  ;;[1 1 1] Move Left/Right
  (Pawn|Input|AddMovementInput _as_bp_player (Transformation|GetActorRightVector _as_bp_player) AxisValue false))

(event Input|AxisEvents|InputAxisMoveForwardBackward
  (params (AxisValue :type Float%20%28single-precision%29))
  (bind _as_bp_player (Variables|Default|GetAs%20BP%20Player))
  ;[1 1 1] Move
  ;;[1 1 1] Move Forward/Backward
  (Pawn|Input|AddMovementInput _as_bp_player (Transformation|GetActorForwardVector _as_bp_player) AxisValue false))

(event Input|AxisEvents|InputAxisRotate
  (params (AxisValue :type Float%20%28single-precision%29))
  ;[1 1 1] Rotate
  (Pawn|Input|AddControllerYawInput (Variables|Default|GetAs%20BP%20Player) AxisValue))

(event Input|AxisEvents|InputAxisLookUp
  (params (AxisValue :type Float%20%28single-precision%29))
  ;[1 1 1] Rotate
  (Pawn|Input|AddControllerPitchInput (Variables|Default|GetAs%20BP%20Player) AxisValue))

(fn ConstructionScript)